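; StoneDown_BP is a falling-stone obstacle, using SMB3 object sprites, that repeatedly moves along a timeline-driven path.
; One second after BeginPlay, DropStone lerps the sprite's relative location between points A and B by the timeline's Speed track, then replays after a short pause.
; Each timeline update also calls ChangingFace, which swaps the face sprite once Speed reaches a high threshold.
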(event Custom|DropStone
  ;[0.5637 1 0.5878] DropStone script
  (bind _speed (Timeline|TimelineAnimation PlayFromStart)
    (:Update
      (Utilities|FlowControl|Sequence
        (:then_0
          (Transformation|SetRelativeLocation (Variables|Default|GetPaperSprite) (Math|Vector|Lerp(Vector) (Variables|Default|GetA) (Variables|Default|GetB) _speed) false false))
        (:then_1
          (CallFunction|ChangingFace))))
    (:Finished
      (Utilities|FlowControl|Delay 0.2)
      ;;[0.5153 0.7721 1] Call DropStone event
      (CallFunction|DropStone))))

(event Custom|ChangingFace
  (bind _papersprite (Variables|Default|GetPaperSprite))
  ;[0.6739 0.2482 1] Changin face
  (if (>= (stale Custom|DropStone _speed) 0.8)
    (Rendering|Components|Sprite|SetSprite _papersprite "/Game/Asset2_Mario/SMB3_Objects_Sprite_388.SMB3_Objects_Sprite_388")
    (else
      (Rendering|Components|Sprite|SetSprite _papersprite "/Game/Asset2_Mario/SMB3_Objects_Sprite_371.SMB3_Objects_Sprite_371"))))

(event EventBeginPlay
  ;[1 1 1] Start
  (Utilities|FlowControl|Delay 1.0)
  ;;[0.2937 0.562 1] Call DropStone event
  (CallFunction|DropStone))

(fn ConstructionScript)