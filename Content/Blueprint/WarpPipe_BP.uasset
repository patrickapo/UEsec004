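; Warp pipe actor that teleports the player to the arrow of a linked target location on a key press.
; Entering its box enables input and arms the warp only for a MyCharacter with Mushroom set.
; Pressing C while armed moves the character there, fades the camera in and disarms after a short delay.
; Any end overlap on the box disables input and disarms the warp.
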(event OnComponentBeginOverlap(Box)
  (params (OverlappedComponent :type Primitive%20Component%20Object%20Reference) (OtherActor :type Actor%20Object%20Reference) (OtherComp :type Primitive%20Component%20Object%20Reference) (OtherBodyIndex :type Integer) (bFromSweep :type Boolean) (SweepResult :type Hit%20Result%20Structure%20%28by%20ref%29))
  ;[1 1 1] Enable Input
  (bind _asmy_character (Utilities|Casting|CastToMyCharacter OtherActor))
  (if (Variables|/Game/Blueprint/MyCharacter.MyCharacter_C|GetMushroom _asmy_character)
    (Development|PrintString "Enable input")
    (Input|EnableInput (Game|GetPlayerController 0))
    (Variables|Default|SetEnableWarp true)))

(event OnComponentEndOverlap(Box)
  (params (OverlappedComponent :type Primitive%20Component%20Object%20Reference) (OtherActor :type Actor%20Object%20Reference) (OtherComp :type Primitive%20Component%20Object%20Reference) (OtherBodyIndex :type Integer))
  ;[0.477 1 0.6007] End overlap then disable input
  (Input|DisableInput (Game|GetPlayerController 0) 0)
  (Variables|Default|SetEnableWarp false)
  (Development|PrintString "Teleport Disabled"))

(event Input|KeyboardEvents|C
  (params (Key :type Key%20Structure :default "None"))
  (:Pressed
    (if (Variables|Default|GetEnableWarp)
      (Transformation|SetWorldLocation (Variables|/Script/Engine.Actor|GetRootComponent (stale OnComponentBeginOverlap(Box) _asmy_character)) (Transformation|GetSocketLocation (Variables|WarpPipe_BP_C|GetArrow (Variables|Default|GetTargetLocation)) "None") false false)
      (Utilities|FlowControl|Sequence
        (:then_0
          (CameraFades|StartCameraFade :self (Game|GetPlayerCameraManager 0) :FromAlpha 1.0 :Duration 2.0)
          (Utilities|FlowControl|Delay 1.0)
          (Variables|Default|SetEnableWarp false)
          (Development|PrintString "Teleport End"))))))

(fn ConstructionScript)