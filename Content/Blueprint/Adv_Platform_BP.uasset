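; One-way sprite or mesh platform that turns solid for the player character and lets it drop through on C.
; UpperBox overlap enables RenderComponent collision, while LowerBox overlap enables the platform's own input for player controller 0.
; Pressing C disables RenderComponent collision, with CollisionStatus tracking the solid state.
; Leaving UpperBox while solid waits briefly, then disables LowerBox collision rather than RenderComponent's and clears the flag.
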(event OnComponentBeginOverlap(UpperBox)
  (params (OverlappedComponent :type Primitive%20Component%20Object%20Reference) (OtherActor :type Actor%20Object%20Reference) (OtherComp :type Primitive%20Component%20Object%20Reference) (OtherBodyIndex :type Integer) (bFromSweep :type Boolean) (SweepResult :type Hit%20Result%20Structure%20%28by%20ref%29))
  ;[0.3769 0.6032 1] Upper Collision
  (Utilities|Casting|CastToMyCharacter OtherActor)
  (if (not (Variables|Default|GetCollisionStatus))
    (Collision|SetCollisionEnabled (Variables|Default|GetRenderComponent) "QueryAndPhysics")
    (Variables|Default|SetCollisionStatus true)))

(event OnComponentBeginOverlap(LowerBox)
  (params (OverlappedComponent :type Primitive%20Component%20Object%20Reference) (OtherActor :type Actor%20Object%20Reference) (OtherComp :type Primitive%20Component%20Object%20Reference) (OtherBodyIndex :type Integer) (bFromSweep :type Boolean) (SweepResult :type Hit%20Result%20Structure%20%28by%20ref%29))
  ;[1 0.477 0.8763] Lower Collision
  (Utilities|Casting|CastToMyCharacter OtherActor)
  (Input|EnableInput (Game|GetPlayerController 0)))

(event OnComponentEndOverlap(UpperBox)
  (params (OverlappedComponent :type Primitive%20Component%20Object%20Reference) (OtherActor :type Actor%20Object%20Reference) (OtherComp :type Primitive%20Component%20Object%20Reference) (OtherBodyIndex :type Integer))
  ;[1 1 1] Fixed bug
  (Utilities|Casting|CastToMyCharacter OtherActor)
  (if (Variables|Default|GetCollisionStatus)
    (Utilities|FlowControl|Delay 0.5)
    (Collision|SetCollisionEnabled (Variables|Default|GetLowerBox) "NoCollision")
    (Variables|Default|SetCollisionStatus false)))

(event Input|KeyboardEvents|C
  (params (Key :type Key%20Structure :default "None"))
  ;[0.5599 1 0.5568] Press C to jump down
  (:Pressed
    (if (Variables|Default|GetCollisionStatus)
      (Collision|SetCollisionEnabled (Variables|Default|GetRenderComponent) "NoCollision")
      (Variables|Default|SetCollisionStatus false))))

(fn ConstructionScript)