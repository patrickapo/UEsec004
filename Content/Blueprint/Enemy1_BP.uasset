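; Enemy1_BP is a 2D Paper2D enemy that walks back and forth on its own.
; Each Tick it moves along its forward vector, records horizontal direction in IsMovingRight and picks the walk or idle flipbook from its velocity.
; A one-second Delay on Tick acts as a repeating timer that rotates the actor 180 degrees, reversing the patrol.
; IsMovingRight is only written here, and BeginPlay sets the flipbook component to replicate.
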(event Custom|DirectionChange
  ;[1 1 1] Direction change
  (if (> (.x (Transformation|GetVelocity)) 0.0)
    (Variables|Default|SetIsMovingRight true)
    (elif (< (.x (Transformation|GetVelocity)) 0.0)
      (Variables|Default|SetIsMovingRight false))))

(event Custom|UpdateAnimation
  ;[1 1 1] Animation
  (Sprite|SetFlipbook (Variables|Default|GetPaperFlipbook) (select (> (Math|Vector|VectorLength (Transformation|GetVelocity)) 0.0) "/Game/Asset3_Flipbooks/Enemy_walk.Enemy_walk" "/Game/Asset3_Flipbooks/Enemy_Idle.Enemy_Idle")))

(event Custom|Movement
  ;[1 1 1] Move Forward
  (Pawn|Input|AddMovementInput (Transformation|GetActorForwardVector) 1.0 false))

(event Custom|Turn%20Char
  ;[1 1 1] Turn Character
  (Transformation|SetActorRotation (Math|Rotator|CombineRotators (Transformation|GetActorRotation) "0.000000,180.000000,0.000000")))

(event EventBeginPlay
  ;[1 1 1] Animation
  (Class|ActorComponent|SetIsReplicated (Variables|Default|GetPaperFlipbook) true))

(event EventTick
  (params (DeltaSeconds :type Float%20%28single-precision%29))
  ;[1 1 1] Start of game
  (Utilities|FlowControl|Sequence
    (:then_0
      (CallFunction|Movement)
      (CallFunction|DirectionChange)
      (CallFunction|UpdateAnimation))
    (:then_1
      (Utilities|FlowControl|Delay 1.0)
      (CallFunction|TurnChar))))

(fn ConstructionScript)